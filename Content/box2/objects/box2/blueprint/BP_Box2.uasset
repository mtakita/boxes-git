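; BP_Box2 is a possessable box object, apparently for a staged game, with its own camera.
; On possession it snaps the camera to the current player camera manager's transform, then eases it to a fixed, angled relative position over half a second for a seamless view transition.
; Initialize, Pressed and Released are stubs: Initialize ignores its stage, difficulty and director inputs, and both input functions return false.
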(event Collision|EventActorBeginOverlap
  (params (OtherActor :type Actor%20Object%20Reference)))

(event EventTick
  (params (DeltaSeconds :type Float%20%28single-precision%29)))

(event EventPossessed
  (params (NewController :type Controller%20Object%20Reference))
  (bind _returnvalue (Game|GetPlayerCameraManager 0))
  (bind _camera (Variables|Default|GetCamera))
  (bind _returnvalue_2 (Transformation|GetActorTransform _returnvalue))
  (Transformation|SetWorldTransform _camera (Math|Transform|MakeTransform (.location _returnvalue_2) (.rotation _returnvalue_2) "1,1,1") false false)
  (Components|MoveComponentTo _camera "35.432514,0.000031,97.349854" "-20.000000, 0, 0" false false 0.5 false))

(fn ConstructionScript)

(fn Initialize
  (params (NumOfStage :type Integer) (Difficulity :type Integer) (DirectorEventUpStream :type I%20Director%20Event%20Up%20Stream%20Interface))
  (return 0))

(fn Pressed
  (return false))

(fn Released
  (return false))