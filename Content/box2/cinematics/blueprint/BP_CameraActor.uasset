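; BP_CameraActor is a cinematic camera actor that plays the intro-to-game Level Sequence.
; On BeginPlay it becomes player 0's view target and plays the sequence, set to pause at its end.
; Initialize stores an upstream director reference, ignoring stage number and difficulty.
; Stage2IntroCameraEnd reports an enum event to that director and returns false.
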(event EventBeginPlay
  (Game|Player|SetViewTargetwithBlend (Game|GetPlayerController 0) self 0.0 "VTBlend_Linear" 0.0 false)
  (bind _returnvalue (Sequencer|Player|CreateLevelSequencePlayer "/Game/box2/cinematics/sequence/cinema_intro_to_game.cinema_intro_to_game" (Utilities|Struct|MakeMovieSceneSequencePlaybackSettings false "(Value=0)" 1.0 0.0 false false false false false false false true)))
  (Sequencer|Player|Play _returnvalue :!class /Script/MovieScene.MovieSceneSequencePlayer))

(event Collision|EventActorBeginOverlap
  (params (OtherActor :type Actor%20Object%20Reference)))

(event EventTick
  (params (DeltaSeconds :type Float%20%28single-precision%29)))

(fn ConstructionScript)

(fn Initialize
  (params (NumOfStage :type Integer) (Difficulity :type Integer) (DirectorEventUpStream :type I%20Director%20Event%20Up%20Stream%20Interface))
  (Variables|Default|SetdirectorUpstream DirectorEventUpStream)
  (return 0))

(fn Stage2IntroCameraEnd
  (params (NewParam :type Boolean))
  (Default|Report (Variables|Default|GetdirectorUpstream) "NewEnumerator15")
  (return false))