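; BP_FlyingText is a flying-text prop actor for the stage 2 "Kanpe 1" event, driven by a director event chain.
; Initialize stores the upstream director, and Report reacts to that event by revealing and unpausing the skeletal mesh and playing the therapy text animation on its ABP_FlyingText.
; On BeginPlay it binds to the anim blueprint's end callback, which reports the event back upstream and destroys the actor.
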(event Custom|CustomEvent_0
  (Default|Report (Variables|Default|GetdirectorEventUpstream) "NewEnumerator14")
  (Actor|DestroyActor))

(event EventBeginPlay
  (bind _asabp_flying_text (Utilities|Casting|CastToABP_FlyingText (Components|SkeletalMesh|GetAnimInstance (Variables|Default|GetSkeletalMesh))))
  (EventDispatchers|BindEventtoAnimationEnd _asabp_flying_text (delegate Custom|CustomEvent_0)))

(event Collision|EventActorBeginOverlap
  (params (OtherActor :type Actor%20Object%20Reference)))

(event EventTick
  (params (DeltaSeconds :type Float%20%28single-precision%29)))

(fn ConstructionScript)

(fn State2kanpe1
  (bind _skeletalmesh (Variables|Default|GetSkeletalMesh))
  (bind _asabp_flying_text (Utilities|Casting|CastToABP_FlyingText (Components|SkeletalMesh|GetAnimInstance _skeletalmesh)))
  (Variables|/Script/Engine.SkeletalMeshComponent|SetbPauseAnims _skeletalmesh false)
  (Rendering|SetVisibility _skeletalmesh true false)
  (Class|AnimInstance|PlaySlotAnimation _asabp_flying_text "/Game/Objects/kanpe/mesh/flyingtext_Anim_Armature_007_therapy.flyingtext_Anim_Armature_007_therapy" "None" 0.25 0.25 1.0 1))

(fn Initialize
  (params (NumOfStage :type Integer) (Difficulity :type Integer) (DirectorEventUpStream :type I%20Director%20Event%20Up%20Stream%20Interface))
  (Variables|Default|SetdirectorEventUpstream DirectorEventUpStream)
  (return 0))

(fn Report
  (params (EventId :type Enum_AllDirectorEvent%20Enum :default "NewEnumerator1"))
  (switch Utilities|FlowControl|Switch|SwitchonEnum_AllDirectorEvent EventId
    (:NewEnumerator14
      (CallFunction|State2kanpe1)
      (return false))))