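; BP_HUD_Stage1_Start is a director-driven event object that shows the Stage 1 start HUD for the Kanpe 1 sequence.
; On receiving the Stage 1 Kanpe 1 1 event through Report, it creates the HUD_Stage1Start widget and adds it to the viewport.
; A three-second named timer then calls Kanpe_1, which removes the widget and reports Stage1_Kanpe1_1 to the upstream director supplied by Initialize.
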(event Custom|Kanpe_1
  (Widget|RemovefromParent (Variables|Default|GetHUD))
  (Default|Report (Variables|Default|GetdirectorEventUpStream) "NewEnumerator11"))

(event EventTick
  (params (DeltaSeconds :type Float%20%28single-precision%29))
  (switch Utilities|FlowControl|Switch|SwitchonEnum_HUD_Status (Variables|Default|GetcurrentStatus)))

(event EventBeginPlay
  (Variables|Default|SetcurrentStatus "NewEnumerator0"))

(fn ConstructionScript)

(fn Initialize
  (params (NumOfStage :type Integer) (Difficulity :type Integer) (DirectorEventUpStream :type I%20Director%20Event%20Up%20Stream%20Interface))
  (Variables|Default|SetnumOfStage NumOfStage)
  (Variables|Default|Setdifficulty Difficulity)
  (Variables|Default|SetdirectorEventUpStream DirectorEventUpStream)
  (Variables|Default|SetcurrentStatus "NewEnumerator0")
  (return self))

(fn Report
  (params (EventId :type Enum_AllDirectorEvent%20Enum :default "NewEnumerator1"))
  (switch Utilities|FlowControl|Switch|SwitchonEnum_AllDirectorEvent EventId
    (:NewEnumerator11
      (Variables|Default|SetcurrentStatus "NewEnumerator1")
      (bind _returnvalue (UserInterface|CreateWidget "/Game/box1/Objects/kanpe1/HUD_Stage1Start.HUD_Stage1Start_C" (Game|GetPlayerController 0)))
      (bind _output_get (Variables|Default|SetHUD _returnvalue))
      (UserInterface|Viewport|AddtoViewport _output_get 0)
      ;[1 1 1] HUDの表示期間が終わると、次に遷移する
      (Utilities|Time|SetTimerbyFunctionName self "Kanpe_1" 3.0)
      (return false))))