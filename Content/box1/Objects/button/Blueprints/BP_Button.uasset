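; BP_Button is a touchable button actor that shows a random starting digit from 0 to 9 and counts it down when tapped.
; The first touch fires ButtonPushed and starts a looping one-second CountDown timer.
; UpdateNumber displays each digit by swapping materials on two mesh slots.
; Below zero, the timer stops and IAMLID-tagged buttons are scanned for any below one, but that result triggers nothing.
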(event OnInputTouchEnd(StaticMeshComponent)
  (params (FingerIndex :type ETouchIndex%20Enum :default "Touch1") (TouchedComponent :type Primitive%20Component%20Object%20Reference))
  ;[1 1 1] ボタンがすでに押されている場合は何もしない
  (if (Variables|Default|GetbuttonUnpushedFlg)
    (Variables|Default|SetbuttonUnpushedFlg false)
    ;[1 1 1] タッチを検出したら数字をカウントダウン開始する
    (bind _returnvalue (Utilities|Time|SetTimerbyFunctionName 0 "CountDown" 1.0 true))
    (Variables|Default|SettimerHandle _returnvalue)
    (Default|CallButtonPushed)
    (Development|PrintString "buttonPushed has been called!!!")))

(event EventBeginPlay
  ;[1 1 1] 最初にボタンに表示する数字をランダムに決める。
  (bind _output_get (Variables|Default|Setnumber (Math|Random|RandomIntegerinRange 0 9)))
  (Development|PrintString (Utilities|String|ToString(Integer) _output_get))
  (CallFunction|UpdateNumber _output_get))

(event Collision|EventActorBeginOverlap
  (params (OtherActor :type Actor%20Object%20Reference)))

(event EventTick
  (params (DeltaSeconds :type Float%20%28single-precision%29)))

(event EventTick
  (params (DeltaSeconds :type Float%20%28single-precision%29)))

(fn ConstructionScript)

(fn CountDown
  ;[1 1 1] 数字をカウントダウンして新しい数字を表示する
  (CallFunction|UpdateNumber (- (Variables|Default|Getnumber) 1))
  (bind _output_get (Variables|Default|Setnumber (- (Variables|Default|Getnumber) 1)))
  (if (< _output_get 0)
    (Utilities|Time|ClearandInvalidateTimerbyHandle (Variables|Default|GettimerHandle))
    (bind _outactors (Actor|GetAllActorswithTag "IAMLID"))
    ;[1 1 1] 四つのボタンがカウントダウンしてしまっているか検証する
    (Variables|Default|Setcountdowned false)
    (for _array_element _outactors
      (bind _asbp_button (Utilities|Casting|CastToBP_Button _array_element))
      (if (< (Variables|BP_Button_C|Getnumber _asbp_button) 1)
        (Variables|Default|Setcountdowned true)))
    (if (Variables|Default|Getcountdowned)
      _)))

(fn UpdateNumber
  (params (newNumber :type Integer))
  (bind _returnvalue (Math|Conversions|ToFloat(Integer) newNumber))
  (bind _staticmesh (Variables|Default|GetStaticMesh))
  ;[1 1 1] 開始直後に表示される数字を決定する。(1-9)
  (Development|PrintString (Utilities|String|ToString(Integer) newNumber))
  (if (<= _returnvalue 0.0)
    (Rendering|Material|SetMaterial _staticmesh 0 "/Game/box1/Objects/button/Materials/M_0_edge_yellow_Mat.M_0_edge_yellow_Mat")
    (Rendering|Material|SetMaterial _staticmesh 2 "/Game/box1/Objects/button/Materials/M_0_edge_yellow_Mat.M_0_edge_yellow_Mat")
    (elif (<= _returnvalue 1.0)
      (Rendering|Material|SetMaterial _staticmesh 0 "/Game/box1/Objects/button/Materials/M_1_edge_yellow_Mat.M_1_edge_yellow_Mat")
      (Rendering|Material|SetMaterial _staticmesh 2 "/Game/box1/Objects/button/Materials/M_1_edge_yellow_Mat.M_1_edge_yellow_Mat")
      (elif (<= _returnvalue 2.0)
        (Rendering|Material|SetMaterial _staticmesh 0 "/Game/box1/Objects/button/Materials/M_2_edge_yellow_Mat.M_2_edge_yellow_Mat")
        (Rendering|Material|SetMaterial _staticmesh 2 "/Game/box1/Objects/button/Materials/M_2_edge_yellow_Mat.M_2_edge_yellow_Mat")
        (elif (<= _returnvalue 3.0)
          (Rendering|Material|SetMaterial _staticmesh 0 "/Game/box1/Objects/button/Materials/M_3_edge_yellow_Mat.M_3_edge_yellow_Mat")
          (Rendering|Material|SetMaterial _staticmesh 2 "/Game/box1/Objects/button/Materials/M_3_edge_yellow_Mat.M_3_edge_yellow_Mat")
          (elif (<= _returnvalue 4.0)
            (Rendering|Material|SetMaterial _staticmesh 0 "/Game/box1/Objects/button/Materials/M_4_edge_yellow_Mat.M_4_edge_yellow_Mat")
            (Rendering|Material|SetMaterial _staticmesh 2 "/Game/box1/Objects/button/Materials/M_4_edge_yellow_Mat.M_4_edge_yellow_Mat")
            (elif (<= _returnvalue 5.0)
              (Rendering|Material|SetMaterial _staticmesh 0 "/Game/box1/Objects/button/Materials/M_5_edge_yellow_Mat.M_5_edge_yellow_Mat")
              (Rendering|Material|SetMaterial _staticmesh 2 "/Game/box1/Objects/button/Materials/M_5_edge_yellow_Mat.M_5_edge_yellow_Mat")
              (elif (<= _returnvalue 6.0)
                (Rendering|Material|SetMaterial _staticmesh 0 "/Game/box1/Objects/button/Materials/M_6_edge_yellow_Mat.M_6_edge_yellow_Mat")
                (Rendering|Material|SetMaterial _staticmesh 2 "/Game/box1/Objects/button/Materials/M_6_edge_yellow_Mat.M_6_edge_yellow_Mat")
                (elif (<= _returnvalue 7.0)
                  (Rendering|Material|SetMaterial _staticmesh 0 "/Game/box1/Objects/button/Materials/M_7_edge_yellow_Mat.M_7_edge_yellow_Mat")
                  (Rendering|Material|SetMaterial _staticmesh 2 "/Game/box1/Objects/button/Materials/M_7_edge_yellow_Mat.M_7_edge_yellow_Mat")
                  (elif (<= _returnvalue 8.0)
                    (Rendering|Material|SetMaterial _staticmesh 0 "/Game/box1/Objects/button/Materials/M_8_edge_yellow_Mat.M_8_edge_yellow_Mat")
                    (Rendering|Material|SetMaterial _staticmesh 2 "/Game/box1/Objects/button/Materials/M_8_edge_yellow_Mat.M_8_edge_yellow_Mat")
                    (else
                      (Rendering|Material|SetMaterial _staticmesh 0 "/Game/box1/Objects/button/Materials/M_9_edge_yellow_Mat.M_9_edge_yellow_Mat")
                      (Rendering|Material|SetMaterial _staticmesh 2 "/Game/box1/Objects/button/Materials/M_9_edge_yellow_Mat.M_9_edge_yellow_Mat"))))))))))))

(fn Pressed
  (return false))

(fn Released
  (return false))