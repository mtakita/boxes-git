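; Touchable box actor that tells taps from swipes, selecting on a tap and rotating itself on a swipe.
; Press records the touch position and actor under the finger, then starts a looping timer that flags a swipe past time or distance thresholds.
; Swipes rotate the box by RotateDelta around the camera-to-box line crossed with the deprojected finger movement.
; Release without swiping stores the hit actor as selected, or calls the selection-switch listener.
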(event Custom|MyCustomEvent
  (bind _returnvalue (Transformation|GetActorRotation))
  (bind (_roll _pitch _yaw) (Math|Rotator|BreakRotator _returnvalue))
  (Transformation|AddActorLocalRotation (Math|Rotator|MakeRotator (+ _roll 2e+01) _pitch _yaw) false false))

(event Custom|Released_ISelectable
  (bind _hitactor (Variables|Default|GetHitActor))
  ;[1 1 1] Measure Time.  Time elapsed is going to be stored in "timeElapsed."
  ;;[1 1 1] タイマー停止
  (Utilities|Time|ClearandInvalidateTimerbyHandle (stale Custom|Pressed_ISelectable _returnvalue_4))
  ;;[1 1 1] タッチ発生検証
  (if (not (Variables|Default|GetEngagingSwipeFlg))
    ;;[1 1 1] タッチ発生
    (Development|PrintString "Touch occurred!!")
    ;[1 1 1] オブジェクトを選択する
    (if (Utilities|IsValid (Variables|Default|GetHitActor))
      (Development|PrintString (Utilities|GetDisplayName _hitactor))
      (Variables|Default|SetSelectedActor _hitactor)
      (else
        (Default|CallSelectionSwitchListener)
        (Development|PrintString "Listener has been called!!!")))))

(event Custom|Pressed_ISelectable
  (params (BP_Camera :type BP%20Camera%20Object%20Reference))
  (bind _returnvalue (Game|GetPlayerController 0))
  (bind _returnvalue_2 (Game|GetPlayerController 0))
  (bind _array (Utilities|Array|MakeArray "ObjectTypeQuery3" "ObjectTypeQuery2" "ObjectTypeQuery1"))
  (bind (_locationx _locationy) (Class|PlayerController|GetInputTouchState _returnvalue "Touch1"))
  (bind (_hitresult _returnvalue_3) (Class|PlayerController|GetHitResultUnderFingerforObjects _returnvalue_2 "Touch1" _array true))
  ;[1 1 1] Measure Time.  Time elapsed is going to be stored in "timeElapsed."
  ;;[1 1 1] 各種変数をクリア
  (Variables|Default|SetEngagingSwipeFlg false)
  (Variables|Default|SetHitActor 0)
  ;;[1 1 1] タイマー開始
  (bind _returnvalue_4 (Utilities|Time|SetTimerbyEvent (delegate Custom|TimeTick_ISelectable) (Variables|Default|GetTouchSensitivity) true))
  ;;[1 1 1] タッチ開始時刻取得
  (Variables|Default|SetTouchBeginTime (Class|KismetSystemLibrary|GetTimerElapsedTimeHandle _returnvalue_4))
  (Variables|Default|SetTouchAccmTime 0.0)
  ;;[1 1 1] タッチ開始位置取得
  (Variables|Default|SetTouchBeginningPos (Math|Vector2D|MakeVector2D _locationx _locationy))
  ;[1 1 1] タッチポイントにあるオブジェクトを調べておく。
  (if _returnvalue_3
    (Variables|Default|SetHitActor (.HitActor (Collision|BreakHitResult _hitresult)))))

(event Custom|TimeTick_ISelectable
  (bind _returnvalue (Game|GetPlayerController 0))
  (bind _returnvalue_2 (Game|GetPlayerController 0))
  (bind _returnvalue_3 (Game|GetPlayerController 0))
  (bind _rotatedelta (Variables|Default|GetrotateDelta))
  (bind (_locationx _locationy) (Class|PlayerController|GetInputTouchState _returnvalue_3 "Touch1"))
  (bind (_locationx_2 _locationy_2) (Class|PlayerController|GetInputTouchState _returnvalue_2 "Touch1"))
  ;[1 1 1] Measure Time.  Time elapsed is going to be stored in "timeElapsed."
  (if (Utilities|Time|IsTimerActivebyHandle (stale Custom|Pressed_ISelectable _returnvalue_4))
    ;;[1 1 1] 経過時間加算
    (bind _output_get (Variables|Default|SetTouchAccmTime (+ (Class|KismetSystemLibrary|GetTimerElapsedTimeHandle (stale Custom|Pressed_ISelectable _returnvalue_4)) (Variables|Default|GetTouchAccmTime))))
    (if (not (and (< (- _output_get (Variables|Default|GetTouchBeginTime)) (Variables|Default|GetTouchTimeThreshold)) (< (Math|Vector|Distance2D(Vector) (Math|Vector2D|MakeVector2D _locationx _locationy) (Variables|Default|GetTouchBeginningPos)) (Variables|Default|GetTouchDistanceThreshold))))
      ;;[1 1 1] Swipe発生
      (Variables|Default|SetEngagingSwipeFlg true)
      (Development|PrintString "Swipe occured!!!")
      ;[1 1 1] Swipe終了Screen座標を記録する
      (Variables|Default|SetTouchEnd2DVector (Math|Vector2D|MakeVector2D _locationx_2 _locationy_2))
      ;[1 1 1] 一定量Swipeされていることを確認
      (if (> (Math|Vector|Distance2D(Vector) (Variables|Default|GetTouchStart2DVector) (Variables|Default|GetTouchEnd2DVector)) 1.0)
        (Transformation|SetActorRotation (Math|Rotator|MakeRotationfromAxes (Math|Vector|RotateVectorAroundAxis (Transformation|GetActorForwardVector) _rotatedelta (Math|Vector|CrossProduct (- (Transformation|GetActorLocation (stale Custom|Pressed_ISelectable BP_Camera)) (Transformation|GetActorLocation)) (- (.WorldPosition (Class|GameplayStatics|DeprojectScreentoWorld _returnvalue (Variables|Default|GetTouchEnd2DVector))) (.WorldPosition (Class|GameplayStatics|DeprojectScreentoWorld _returnvalue (Variables|Default|GetTouchStart2DVector)))))) (Math|Vector|RotateVectorAroundAxis (Transformation|GetActorRightVector) _rotatedelta (Math|Vector|CrossProduct (- (Transformation|GetActorLocation (stale Custom|Pressed_ISelectable BP_Camera)) (Transformation|GetActorLocation)) (- (.WorldPosition (Class|GameplayStatics|DeprojectScreentoWorld _returnvalue (Variables|Default|GetTouchEnd2DVector))) (.WorldPosition (Class|GameplayStatics|DeprojectScreentoWorld _returnvalue (Variables|Default|GetTouchStart2DVector)))))) (Math|Vector|RotateVectorAroundAxis (Transformation|GetActorUpVector) _rotatedelta (Math|Vector|CrossProduct (- (Transformation|GetActorLocation (stale Custom|Pressed_ISelectable BP_Camera)) (Transformation|GetActorLocation)) (- (.WorldPosition (Class|GameplayStatics|DeprojectScreentoWorld _returnvalue (Variables|Default|GetTouchEnd2DVector))) (.WorldPosition (Class|GameplayStatics|DeprojectScreentoWorld _returnvalue (Variables|Default|GetTouchStart2DVector))))))))
        ;[1 1 1] 次のSwipe開始Screen座標はSwipe終了Screen座標となる
        (Variables|Default|SetTouchStart2DVector (Variables|Default|GetTouchEnd2DVector))))))

(event EventBeginPlay)

(event Collision|EventActorBeginOverlap
  (params (OtherActor :type Actor%20Object%20Reference)))

(fn ConstructionScript)

(fn Pressed
  (CallFunction|PressedISelectable)
  (return false))

(fn Released
  (CallFunction|ReleasedISelectable)
  (return false))