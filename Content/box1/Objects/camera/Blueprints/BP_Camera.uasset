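; Stage camera actor that plays a timed fly-around along BP_CameraSplinePath while facing the world origin.
; Report starts the Stage 1 shot, Tick advances it by elapsed time, then reports completion to the upstream director passed to Initialize.
; Tick also rebinds a selection-switch listener every frame, whose handler clears SelectedActor.
; Touch select and swipe-orbit logic remains in the graph but is disconnected and never runs.
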(event Custom|カスタムイベント_1
  ;[1 1 1] 選択をLevel Blueprintに戻す
  (Development|PrintString "Hello")
  (Variables|Default|SetselectedActor 0))

(event Custom|TimerTickReceiver)

(event EventBeginPlay
  (Variables|Default|SetcurrentStatus "NewEnumerator0")
  ;[1 1 1] スプラインを探して持ってくる
  (bind _returnvalue (Actor|GetActorOfClass "/Game/box1/Objects/camera/Blueprints/BP_CameraSplinePath.BP_CameraSplinePath_C"))
  (bind _output_get (Variables|Default|SetsplinePath _returnvalue))
  (Variables|/Script/Engine.SplineComponent|SetDuration (Variables|/Game/box1/Objects/camera/Blueprints/BP_CameraSplinePath.BP_CameraSplinePath_C|GetSpline _output_get) (Variables|Default|GetfukanDuration))
  ;[1 1 1] カメラの初期位置をスプラインの端に合わせる
  (Transformation|SetActorLocation (Spline|GetLocationatTime (Variables|/Game/box1/Objects/camera/Blueprints/BP_CameraSplinePath.BP_CameraSplinePath_C|GetSpline (Variables|Default|GetsplinePath)) 0.0 "World" false) false false)
  (Transformation|SetWorldRotation (Variables|Default|GetCamera) (Math|Rotator|FindLookatRotation (Transformation|GetWorldLocation (Variables|Default|GetCamera)) (Math|Conversions|ToVector(Float) (Class|GameplayStatics|GetWorldOriginLocation))) false false))

(event EventTick
  (params (DeltaSeconds :type Float%20%28single-precision%29))
  (Utilities|FlowControl|Sequence
    (:then_0
      (switch Utilities|FlowControl|Switch|SwitchonEnum_Camera_Status (Variables|Default|GetcurrentStatus)
        (:NewEnumerator1
          ;[1 1 1] Camera_1のイベント
          (bind _output_get (Variables|Default|SetfukaCurrentTimelapse (+ DeltaSeconds (Variables|Default|GetfukaCurrentTimelapse))))
          (Transformation|SetActorLocation (Spline|GetLocationatTime (Variables|/Game/box1/Objects/camera/Blueprints/BP_CameraSplinePath.BP_CameraSplinePath_C|GetSpline (Variables|Default|GetsplinePath)) _output_get "World" false) false false)
          (Transformation|SetWorldRotation (Variables|Default|GetCamera) (Math|Rotator|FindLookatRotation (Transformation|GetWorldLocation (Variables|Default|GetCamera)) (Math|Conversions|ToVector(Float) (Class|GameplayStatics|GetWorldOriginLocation))) false false)
          (if (<= (Variables|Default|GetfukanDuration) (Variables|Default|GetfukaCurrentTimelapse))
            ;;[1 1 1] Camera_1のイベント終了
            (Default|Report (Variables|Default|GetdirectorEventUpStream) "NewEnumerator3")
            (Variables|Default|SetcurrentStatus "NewEnumerator0")))))
    (:then_1
      ;[1 1 1] 選択をLevel Blueprintに戻す
      (EventDispatchers|BindEventtoSelectionSwitchListener 0 (delegate Custom|カスタムイベント_1)))))

(event Input|ActionEvents|InputActionFinger1
  (params (Key :type Key%20Structure :default "None")))

(fn ConstructionScript)

(fn Initialize
  (params (NumOfStage :type Integer) (Difficulity :type Integer) (DirectorEventUpStream :type I%20Director%20Event%20Up%20Stream%20Interface))
  (Variables|Default|SetnumOfStage NumOfStage)
  (Variables|Default|Setdifficulty Difficulity)
  (Variables|Default|SetdirectorEventUpStream DirectorEventUpStream)
  (Variables|Default|SetcurrentStatus "NewEnumerator0")
  (return self))

(fn Report
  (params (EventId :type Enum_AllDirectorEvent%20Enum :default "NewEnumerator1"))
  (switch Utilities|FlowControl|Switch|SwitchonEnum_AllDirectorEvent EventId
    (:NewEnumerator3
      ;[1 1 1] Camera_1のイベント初期化
      (Variables|Default|SetcurrentStatus "NewEnumerator1")
      (Variables|Default|SetfukaCurrentTimelapse 0.0)
      (Variables|Default|SetfukanSpeed (/ (Spline|GetSplineLength (Actor|GetComponentbyClass (Variables|Default|GetsplinePath) "/Script/Engine.SplineComponent")) (Variables|Default|GetfukanDuration)))
      (return false))))