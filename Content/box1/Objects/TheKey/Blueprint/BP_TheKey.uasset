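; BP_TheKey is a key actor that exchanges stage 1 events with an upstream director supplied through Initialize, along with stage number and difficulty.
; Report stores incoming key events in CurrentEvent, which Tick acts on as a simple state machine.
; Key 1 is a debug step echoed straight back upstream.
; Key 2 watches for the mesh falling below a height limit, then reports Key 3 and destroys the actor.
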(event EventBeginPlay)

(event Collision|EventActorBeginOverlap
  (params (OtherActor :type Actor%20Object%20Reference)))

(event EventTick
  (params (DeltaSeconds :type Float%20%28single-precision%29))
  (switch Utilities|FlowControl|Switch|SwitchonEnum_AllDirectorEvent (Variables|Default|GetcurrentEvent)
    (:NewEnumerator8
      ;[1 1 1] デバック用
      (Variables|Default|SetcurrentEvent "NewEnumerator1")
      (Default|Report (Variables|Default|GetdirectorEventUpStream) "NewEnumerator8"))
    (:NewEnumerator9
      ;[1 1 1] 鍵の落下判定
      (if (<= (.z (Transformation|GetWorldLocation (Variables|Default|GetStaticMesh self))) -3e+03)
        (Default|Report (Variables|Default|GetdirectorEventUpStream) "NewEnumerator10")
        ;[1 1 1] アクターを破棄する
        (Actor|DestroyActor)))))

(fn ConstructionScript)

(fn Initialize
  (params (NumOfStage :type Integer) (Difficulity :type Integer) (DirectorEventUpStream :type I%20Director%20Event%20Up%20Stream%20Interface))
  (Variables|Default|SetnumOfStage NumOfStage)
  (Variables|Default|Setdifficulty Difficulity)
  (Variables|Default|SetdirectorEventUpStream DirectorEventUpStream)
  (return self))

(fn Report
  (params (EventId :type Enum_AllDirectorEvent%20Enum :default "NewEnumerator1"))
  (switch Utilities|FlowControl|Switch|SwitchonEnum_AllDirectorEvent EventId
    (:NewEnumerator8
      (Variables|Default|SetcurrentEvent "NewEnumerator8"))
    (:NewEnumerator9
      (Variables|Default|SetcurrentEvent "NewEnumerator9")))
  (return false))